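; BP_Canvas is a paint-test actor that serves as a canvas built from a configurable mesh and material.
; On BeginPlay it applies the mesh and material to its StaticMesh component, then passes that component to the BPACCanvas component through SetCanvas.
; An Update event reruns the same setup, and the construction script is empty.
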(event `self.ReceiveBeginPlay`
  (`|ExecutionSequence` :!label _label
    (:`then_0`
      (`StaticMeshComponent.SetStaticMesh` (`self.StaticMesh`) (`self.Mesh`)))
    (:`then_1`
      (`PrimitiveComponent.SetMaterial` (`self.StaticMesh`) 0 (`self.Material`)))
    (:`then_2`
      (`/Game/BP/BP_AC_Canvas.SetCanvas` (`self.BP_AC_Canvas`) (`self.StaticMesh`)))))

(event `Update`
  (goto _label))

(fn `UserConstructionScript`)