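; Chess board actor with an inspection event inherited from its parent, whose chess pawn can be taken as an item.
; TakePawn adds an item through the detective controller, then plays a timeline that flies the pawn component toward a point above the player and destroys it when finished.
; Each update lerps from the pawn's current location to the player's live position, so the motion compounds and follows the player.
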(event `self.ReceiveBeginPlay`
  (`parent.ReceiveBeginPlay`))

(event `self.ReceiveActorBeginOverlap`
  (params (OtherActor :type "Actor Object Reference"))
  (`parent.ReceiveActorBeginOverlap` OtherActor))

(event `self.ReceiveTick`
  (params (DeltaSeconds :type "Float (single-precision)"))
  (`parent.ReceiveTick` DeltaSeconds))

(event `/Game/BP/BPI_Interactable.StartInspection`
  (`parent.StartInspection`))

(event `TakePawn`
  (bind _chesspawn (`self.ChessPawn`))
  (bind (_returnvalue_x _returnvalue_y _returnvalue_z) (`KismetMathLibrary.BreakVector` (`self.K2_GetActorLocation` (`GameplayStatics.GetPlayerPawn` 0))))
  (`/Game/Player/BP/BP_PlayerController.AddItem` (`/Game/BP/BPL_General.GetDetectiveController`) "NewEnumerator1")
  (bind (_direction _alpha) (`Timeline|Timeline_0` :!via `PlayFromStart`)
    (:`Update`
      (`SceneComponent.K2_SetWorldTransform` _chesspawn (`KismetMathLibrary.MakeTransform` (`KismetMathLibrary.VLerp` (`SceneComponent.K2_GetComponentLocation` _chesspawn) (`KismetMathLibrary.MakeVector` _returnvalue_x _returnvalue_y (+ _returnvalue_z 100.0)) _alpha) (struct) (0.7 0.7 0.7)) false false))
    (:`Finished`
      (`ActorComponent.K2_DestroyComponent` (`self.ChessPawn`)))))

(fn `UserConstructionScript`
  (`parent.UserConstructionScript`))