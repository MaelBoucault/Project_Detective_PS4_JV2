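; Magnifying glass actor that follows the mouse cursor in the world and faces the camera.
; On BeginPlay, the glass mesh is hidden from the main pass and written only to custom depth.
; A fast looping timer traces behind the glass, deriving its camera distance from close hits or otherwise restoring the default maximum.
; Tick deprojects the cursor and places the glass along that ray at this distance.
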(event `self.ReceiveBeginPlay`
  (bind _sm_magnifyingglass_glasspart (`self.SM_MagnifyingGlass_GlassPart`))
  (`|ExecutionSequence`
    (:`then_0`
      (`PrimitiveComponent.SetRenderCustomDepth` _sm_magnifyingglass_glasspart true)
      (`PrimitiveComponent.SetRenderInMainPass` _sm_magnifyingglass_glasspart false))
    (:`then_1`
      (`KismetSystemLibrary.K2_SetTimerDelegate` (delegate `AdjustGlassPos`) 0.033 true))))

(event `AdjustGlassPos`
  (bind _returnvalue (`self.K2_GetActorLocation`))
  ; Adjust glass position
  (bind (_outhit _returnvalue_2) (`KismetSystemLibrary.LineTraceSingle` :`Start` _returnvalue :`End` (+ _returnvalue (* (`self.GetActorForwardVector`) -400.0)) :`TraceChannel` "TraceTypeQuery1" :`DrawTime` 2.0))
  (if _returnvalue_2
    (bind (_bblockinghit _binitialoverlap _time _distance) (`GameplayStatics.BreakHitResult` _outhit))
    (if (< _distance 100.0)
      (set `self.DistanceToCamera` (* _distance 0.7))
      (else
        (set `self.DistanceToCamera` (`self.DefaultMaxDistanceToCamera`) :!label _label)))
    (else
      (goto _label))))

(event `self.ReceiveTick`
  (params (DeltaSeconds :type "Float (single-precision)"))
  (`|ExecutionSequence`
    (:`then_0`
      (bind _returnvalue (`WidgetLayoutLibrary.GetMousePositionOnViewport`))
      (bind (_worldposition _worlddirection) (`GameplayStatics.DeprojectScreenToWorld` (`GameplayStatics.GetPlayerController` 0) (* _returnvalue (`WidgetLayoutLibrary.GetViewportScale`))))
      (`SceneComponent.K2_SetWorldLocationAndRotation` (`self.DefaultSceneRoot`) (+ _worldposition (* _worlddirection (`self.DistanceToCamera`))) (`KismetMathLibrary.FindLookAtRotation` (`self.K2_GetActorLocation`) _worldposition) false false))))

(fn `UserConstructionScript`)