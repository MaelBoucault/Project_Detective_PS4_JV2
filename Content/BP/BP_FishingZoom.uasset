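; BP_FishingZoom is a trigger zone that lets the detective pawn fish in front of an open window.
; On box overlap by the detective, it checks that the linked Window is open, then flags the controller and shows the interact prompt on the HUD.
; Leaving the box clears the flag, stops fishing and hides the prompt.
; The window state is only checked on entry, and a missing Window prints a warning.
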(event `self.Box.OnComponentBeginOverlap`
  (params (OverlappedComponent :type "PrimitiveComponent Object Reference") (OtherActor :type "Actor Object Reference") (OtherComp :type "PrimitiveComponent Object Reference") (OtherBodyIndex :type Integer) (bFromSweep :type Boolean) (SweepResult :type "HitResult Structure (by ref)"))
  (if (== (`/Game/BP/BPL_General.GetDetectivePawn`) OtherActor)
    (set `self.PlayerIsHere` true)
    (bind _can (`self.CanFishing`))
    (if _can
      (set `/Game/Player/BP/BP_PlayerController.IsFrontOfOpenWindow` true (`/Game/BP/BPL_General.GetDetectiveController`))
      (`/Game/UI/WBP_BaseHUD.StartShowInteract` (`/Game/BP/BPL_General.GetDetectiveHUD`) true false))))

(event `self.Box.OnComponentEndOverlap`
  (params (OverlappedComponent :type "PrimitiveComponent Object Reference") (OtherActor :type "Actor Object Reference") (OtherComp :type "PrimitiveComponent Object Reference") (OtherBodyIndex :type Integer))
  (if (== (`/Game/BP/BPL_General.GetDetectivePawn`) OtherActor)
    (set `self.PlayerIsHere` false)
    (set `/Game/Player/BP/BP_PlayerController.IsFrontOfOpenWindow` false (`/Game/BP/BPL_General.GetDetectiveController`))
    (`/Game/Player/BP/BP_DetectivePawn.StopFishing` (`/Game/BP/BPL_General.GetDetectivePawn`))
    (`/Game/UI/WBP_BaseHUD.StopShowInteract` (`/Game/BP/BPL_General.GetDetectiveHUD`))))

(fn `CanFishing`
  (returns (Can :type Boolean))
  (bind _window (`self.window`)
    (:`then`
      (return (and (`/Game/BP/Drawer/BP_Windows.Open_0` _window) (`self.PlayerIsHere`))))
    (:`else`
      (`KismetSystemLibrary.PrintString` "FishingZoom Don't Have windowsActor"))))

(fn `UserConstructionScript`)