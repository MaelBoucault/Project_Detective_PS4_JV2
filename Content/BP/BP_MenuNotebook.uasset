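; Notebook menu actor that shows a main page (Resume, Options, Exit) and an options page (Audio, Inputs, Language, Back) built from components.
; Custom events switch pages and show or hide the key-bindings and brush size/color panels by toggling visibility, tracking state in InOption, InInputs and InPinceau.
; A single Select component moves to preset positions to highlight main-page entries.
; Menu hides both sub-panels but resets only InOption.
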(event `NoneSelect`
  (`SceneComponent.SetVisibility` (`self.Select`) false false))

(event `Select_Exit`
  (bind _select (`self.Select`))
  (`SceneComponent.K2_SetRelativeLocation` _select (-13.0 0.0 -7.7) false false)
  (`SceneComponent.SetVisibility` _select true false))

(event `Select_Option`
  (bind _select (`self.Select`))
  (`SceneComponent.K2_SetRelativeLocation` _select (-10.0 0.0 0.5) false false)
  (`SceneComponent.SetVisibility` _select true false))

(event `Select_Resume`
  (bind _select (`self.Select`))
  (`SceneComponent.K2_SetRelativeLocation` _select (-11.0 0.0 8.0) false false)
  (`SceneComponent.SetVisibility` _select true false))

(event `self.ReceiveBeginPlay`
  (set `self.InOption` false)
  (`SceneComponent.SetVisibility` (`self.Select`) false false)
  (`SceneComponent.SetVisibility` (`self.AudioLogo`) false false)
  (`SceneComponent.SetVisibility` (`self.Audio`) false false)
  (`SceneComponent.SetVisibility` (`self.InputsLogo`) false false)
  (`SceneComponent.SetVisibility` (`self.Inputs`) false false)
  (`SceneComponent.SetVisibility` (`self.LanguageLogo`) false false)
  (`SceneComponent.SetVisibility` (`self.Language`) false false)
  (`SceneComponent.SetVisibility` (`self.Back`) false false)
  (`SceneComponent.SetVisibility` (`self.Touches`) false false)
  (`SceneComponent.SetVisibility` (`self.TaillePinceau`) false false)
  (`SceneComponent.SetVisibility` (`self.ColorPinceau`) false false)
  (`SceneComponent.SetVisibility` (`self.ColorPinceau2`) false false)
  (`SceneComponent.SetVisibility` (`self.ColorPinceau1`) false false)
  (`SceneComponent.SetVisibility` (`self.check`) false false)
  (`SceneComponent.K2_SetRelativeLocation` (`self.check`) (-4.0 8.5 9.0) false false))

(event `Options`
  (bind _back (`self.Back`))
  (bind (_relativescale3d_x _relativescale3d_y _relativescale3d_z) (`KismetMathLibrary.BreakVector` (`SceneComponent.RelativeScale3D` _back)))
  (`SceneComponent.SetVisibility` (`self.ExitLogo`) false false)
  (`SceneComponent.SetVisibility` (`self.Exit`) false false)
  (`SceneComponent.SetVisibility` (`self.ResumeLogo`) false false)
  (`SceneComponent.SetVisibility` (`self.Resume`) false false)
  (`SceneComponent.SetVisibility` (`self.Option`) false false)
  (`SceneComponent.SetVisibility` (`self.OptionLogo`) false false)
  (`SceneComponent.SetVisibility` (`self.AudioLogo`) true false)
  (`SceneComponent.SetVisibility` (`self.Audio`) true false)
  (`SceneComponent.SetVisibility` (`self.InputsLogo`) true false)
  (`SceneComponent.SetVisibility` (`self.Inputs`) true false)
  (`SceneComponent.SetVisibility` (`self.LanguageLogo`) true false)
  (`SceneComponent.SetVisibility` (`self.Language`) true false)
  (`SceneComponent.SetVisibility` _back true false)
  (`SceneComponent.SetRelativeScale3D` _back (`KismetMathLibrary.MakeVector` 0.04 _relativescale3d_y _relativescale3d_z))
  (set `self.InOption` true))

(event `Menu`
  (`SceneComponent.SetVisibility` (`self.ExitLogo`) true false)
  (`SceneComponent.SetVisibility` (`self.Exit`) true false)
  (`SceneComponent.SetVisibility` (`self.ResumeLogo`) true false)
  (`SceneComponent.SetVisibility` (`self.Resume`) true false)
  (`SceneComponent.SetVisibility` (`self.Option`) true false)
  (`SceneComponent.SetVisibility` (`self.OptionLogo`) true false)
  (`SceneComponent.SetVisibility` (`self.AudioLogo`) false false)
  (`SceneComponent.SetVisibility` (`self.Audio`) false false)
  (`SceneComponent.SetVisibility` (`self.InputsLogo`) false false)
  (`SceneComponent.SetVisibility` (`self.Inputs`) false false)
  (`SceneComponent.SetVisibility` (`self.LanguageLogo`) false false)
  (`SceneComponent.SetVisibility` (`self.Language`) false false)
  (`SceneComponent.SetVisibility` (`self.Back`) false false)
  (`SceneComponent.SetVisibility` (`self.Touches`) false false)
  (`SceneComponent.SetVisibility` (`self.TaillePinceau`) false false)
  (`SceneComponent.SetVisibility` (`self.ColorPinceau`) false false)
  (`SceneComponent.SetVisibility` (`self.ColorPinceau2`) false false)
  (`SceneComponent.SetVisibility` (`self.ColorPinceau1`) false false)
  (`SceneComponent.SetVisibility` (`self.check`) false false)
  (set `self.InOption` false))

(event `ShowInputs`
  (`SceneComponent.SetVisibility` (`self.Touches`) true false)
  (set `self.InInputs` true))

(event `UnshowInputs`
  (`SceneComponent.SetVisibility` (`self.Touches`) false false)
  (set `self.InInputs` false))

(event `Pinceau`
  (`SceneComponent.SetVisibility` (`self.ColorPinceau`) true false)
  (`SceneComponent.SetVisibility` (`self.TaillePinceau`) true false)
  (`SceneComponent.SetVisibility` (`self.ColorPinceau1`) true false)
  (`SceneComponent.SetVisibility` (`self.ColorPinceau2`) true false)
  (`SceneComponent.SetVisibility` (`self.check`) true false)
  (set `self.InPinceau` true))

(event `PasPinceau`
  (`SceneComponent.SetVisibility` (`self.ColorPinceau`) false false)
  (`SceneComponent.SetVisibility` (`self.TaillePinceau`) false false)
  (`SceneComponent.SetVisibility` (`self.ColorPinceau1`) false false)
  (`SceneComponent.SetVisibility` (`self.ColorPinceau2`) false false)
  (`SceneComponent.SetVisibility` (`self.check`) false false)
  (set `self.InPinceau` false))

(fn `UserConstructionScript`)