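; Inspectable drawing actor (Timeo drawing 02) that toggles between two states when inspection starts, shifting vertically by a fixed offset.
; StartInspection calls Anim, which checks IsOpen to either raise the actor and play SMDrawings reversed from the end, or lower it and set that component's start time offset.
; After raising, a delay re-invokes Anim to lower it automatically if still open.
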(event `self.ReceiveBeginPlay`
  (`parent.ReceiveBeginPlay`))

(event `self.ReceiveActorBeginOverlap`
  (params (OtherActor :type "Actor Object Reference"))
  (`parent.ReceiveActorBeginOverlap` OtherActor))

(event `self.ReceiveTick`
  (params (DeltaSeconds :type "Float (single-precision)"))
  (`parent.ReceiveTick` DeltaSeconds))

(event `Anim`
  (bind (_returnvalue_x _returnvalue_y _returnvalue_z) (`KismetMathLibrary.BreakVector` (`self.K2_GetActorLocation`)))
  (bind (_returnvalue_x_2 _returnvalue_y_2 _returnvalue_z_2) (`KismetMathLibrary.BreakVector` (`self.K2_GetActorLocation`)))
  (bind _sm_drawings (`self.SM_Drawings`))
  (`self.IsOpen`
    (:`then`
      (`self.K2_SetActorLocation` (`KismetMathLibrary.MakeVector` _returnvalue_x_2 _returnvalue_y_2 (- _returnvalue_z_2 40.0)))
      (`GeometryCacheComponent.SetStartTimeOffset` _sm_drawings 2.0)
      (set `self.IsOpen` false))
    (:`else`
      (`self.K2_SetActorLocation` (`KismetMathLibrary.MakeVector` _returnvalue_x _returnvalue_y (+ _returnvalue_z 40.0)))
      (`GeometryCacheComponent.PlayReversedFromEnd` _sm_drawings)
      (set `self.IsOpen` true)
      (`KismetSystemLibrary.Delay` 7.5)
      (`self.IsOpen`
        (:`then`
          (`self.Anim`))
        (:`else`)))))

(event `self.StartInspection`
  (`self.Anim`))

(fn `UserConstructionScript`
  (`parent.UserConstructionScript`))