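; BP_GetShotgun is a trigger volume that marks where the detective can try to get the shotgun at an open window.
; On entering the Box with the linked Window open, it shows the "E" interact prompt and sets the controller's InFrontOfOpenWindow flag.
; Leaving clears both and stops the detective's fishing action.
; CanTryToGetShotgun reports whether the player is present and the window is open.
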(event `self.Box.OnComponentBeginOverlap`
  (params (OverlappedComponent :type "PrimitiveComponent Object Reference") (OtherActor :type "Actor Object Reference") (OtherComp :type "PrimitiveComponent Object Reference") (OtherBodyIndex :type Integer) (bFromSweep :type Boolean) (SweepResult :type "HitResult Structure (by ref)"))
  (bind _returnvalue (== (`/Game/BP/BPL_General.GetDetectivePawn`) OtherActor))
  (set `self.PlayerIsHere` _returnvalue)
  (if (and _returnvalue (`self.GetIsOpenWindow`))
    (`/Game/UI/WBP_BaseHUD.StartShowInteract` (`/Game/BP/BPL_General.GetDetectiveHUD`) (make `/Game/UI/Struct/F_InputInteraction` "E"))
    (set `/Game/Player/BP/BP_PlayerController.InFrontOfOpenWindow` true (`/Game/BP/BPL_General.GetDetectiveController`))))

(event `self.Box.OnComponentEndOverlap`
  (params (OverlappedComponent :type "PrimitiveComponent Object Reference") (OtherActor :type "Actor Object Reference") (OtherComp :type "PrimitiveComponent Object Reference") (OtherBodyIndex :type Integer))
  (bind _detective_pawn (`/Game/BP/BPL_General.GetDetectivePawn`))
  (if (== _detective_pawn OtherActor)
    (set `self.PlayerIsHere` false)
    (`/Game/UI/WBP_BaseHUD.StopShowInteract` (`/Game/BP/BPL_General.GetDetectiveHUD`))
    (set `/Game/Player/BP/BP_PlayerController.InFrontOfOpenWindow` false (`/Game/BP/BPL_General.GetDetectiveController`))
    (`/Game/Player/BP/BP_DetectivePawn.StopFishing` _detective_pawn)))

(fn `CanTryToGetShotgun`
  (returns (Can :type Boolean))
  (return (and (`self.GetIsOpenWindow`) (`self.PlayerIsHere`))))

(fn `GetIsOpenWindow`
  (returns (WindowIsOpen :type Boolean))
  (bind _window (`self.Window`)
    (:`then`
      (bind _output_get (set `self.WindowIsOpen` (`/Game/BP/Drawer/BP_Windows.Open_0` _window)))
      (return _output_get))
    (:`else`
      (`KismetSystemLibrary.PrintString` "YA PAS DE WINDOW LA"))))

(fn `UserConstructionScript`)