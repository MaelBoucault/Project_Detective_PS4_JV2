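; BP_Doors is a door actor that signals when the detective player can interact with it.
; A Box trigger filters overlaps to the detective pawn, showing the E-key interact prompt on the detective HUD on entry and hiding it on exit.
; The same events set and clear IsfrontOfDoor on the detective controller; the door itself holds no opening logic.
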(event `self.Box.OnComponentBeginOverlap`
  (params (OverlappedComponent :type "PrimitiveComponent Object Reference") (OtherActor :type "Actor Object Reference") (OtherComp :type "PrimitiveComponent Object Reference") (OtherBodyIndex :type Integer) (bFromSweep :type Boolean) (SweepResult :type "HitResult Structure (by ref)"))
  (if (== (`/Game/BP/BPL_General.GetDetectivePawn`) OtherActor)
    (`/Game/UI/WBP_BaseHUD.StartShowInteract` (`/Game/BP/BPL_General.GetDetectiveHUD`) true false)
    (set `/Game/Player/BP/BP_PlayerController.IsfrontOfDoor` true (`/Game/BP/BPL_General.GetDetectiveController`))))

(event `self.Box.OnComponentEndOverlap`
  (params (OverlappedComponent :type "PrimitiveComponent Object Reference") (OtherActor :type "Actor Object Reference") (OtherComp :type "PrimitiveComponent Object Reference") (OtherBodyIndex :type Integer))
  (if (== (`/Game/BP/BPL_General.GetDetectivePawn`) OtherActor)
    (`/Game/UI/WBP_BaseHUD.StopShowInteract` (`/Game/BP/BPL_General.GetDetectiveHUD`))
    (set `/Game/Player/BP/BP_PlayerController.IsfrontOfDoor` false (`/Game/BP/BPL_General.GetDetectiveController`))))

(fn `UserConstructionScript`)