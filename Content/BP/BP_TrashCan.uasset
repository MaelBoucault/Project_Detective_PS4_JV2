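; BP_TrashCan is an inspectable trash can holding two drawings that can be taken out one at a time.
; Init maps each collision sphere to an index into parallel drawing arrays, which TakeDrawing uses to select one.
; Taking plays a timeline that moves the drawing and reverses that drawing's own animation.
; A second take or StopInspection triggers Reset, which plays both back and restores the saved transform after a delay.
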(event `self.ReceiveBeginPlay`
  (`parent.ReceiveBeginPlay`)
  (`self.init`)
  (set `self.T01` (`SceneComponent.GetRelativeTransform` (`self.Drawing01`)))
  (set `self.T02` (`SceneComponent.GetRelativeTransform` (`self.Drawing02`))))

(event `TakeDrawing`
  (params (SphereCollision :type "PrimitiveComponent Object Reference"))
  (`self.HasTakeDrawing`
    (:`then`
      (`self.Reset`))
    (:`else`
      (bind _index (`self.GetIndexbycollision` SphereCollision))
      (bind _sucsess (`self.SetCurrentDrawingByIndex` _index))
      (if _sucsess
        (`TimelineComponent.PlayFromStart` (`self.TakeDrawingAnim`))
        (`GeometryCacheComponent.PlayReversedFromEnd` (`|GetArrayItem` (`self.Drawings`) (`self.Index`)))
        (set `self.HasTakeDrawing` true)))))

(event `Reset`
  (bind _takedrawinganim (`self.TakeDrawingAnim`))
  (bind _currentdrawing (`self.CurrentDrawing`))
  (`|ExecutionSequence`
    (:`then_0`
      (`GeometryCacheComponent.PlayFromStart` (`|GetArrayItem` (`self.Drawings`) (`self.Index`)))
      (`TimelineComponent.ReverseFromEnd` _takedrawinganim)
      (`KismetSystemLibrary.Delay` (`TimelineComponent.GetTimelineLength` _takedrawinganim))
      (if (== (`self.Index`) 0)
        (`SceneComponent.K2_SetRelativeTransform` _currentdrawing (`self.T01`) false false)
        (else
          (`SceneComponent.K2_SetRelativeTransform` _currentdrawing (`self.T02`) false false))))
    (:`then_1`
      (set `self.HasTakeDrawing` false))))

(event `/Game/BP/BPI_Interactable.StopInspection`
  (`parent.StopInspection`)
  (`self.Reset`))

(fn `GetIndexbycollision`
  (params (Collision :type "Object Object Reference"))
  (returns (Index :type Integer))
  (bind (_keypin _valuepin) (`|MapForEach` (`self.Collision`))
    (:`then`
      (if (== _keypin Collision)
        (return _valuepin)))
    (:`CompletedPin`
      (`KismetSystemLibrary.PrintString` "INDEX NOT FIND"))))

(fn `init`
  (bind _drawingsscene (`self.DrawingsScene`))
  (bind _drawings (`self.Drawings`))
  (bind _collision (`self.Collision`))
  (`KismetArrayLibrary.Array_Add` _drawingsscene (`self.Drawing01`))
  (`KismetArrayLibrary.Array_Add` _drawingsscene (`self.Drawing02`))
  (`BlueprintMapLibrary.Map_Add` _collision (`self.Sphere01`))
  (`BlueprintMapLibrary.Map_Add` _collision (`self.Sphere02`) 1)
  (`KismetArrayLibrary.Array_Add` _drawings (`self.SM_Drawings1`))
  (`KismetArrayLibrary.Array_Add` _drawings (`self.SM_Drawings2`)))

(fn `SetCurrentDrawingByIndex`
  (params (Index :type Integer))
  (returns (Sucsess :type Boolean))
  (bind _output (`|GetArrayItem` (`self.DrawingsScene`) Index))
  (set `self.Index` Index)
  (`/Engine/EditorBlueprintResources/StandardMacros.IsValid` _output
    (:`Is Valid`
      (set `self.CurrentDrawing` _output)
      (return true))
    (:`Is Not Valid`
      (`KismetSystemLibrary.PrintString` "DRAWING DOSN'T FIND")
      (return false))))

(fn `UserConstructionScript`
  (`parent.UserConstructionScript`))