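; BP_InteractableObject is a data-driven world object that can be highlighted, inspected and may carry a clue.
; Update looks up data by ObjectName, sets the mesh, sizes and pushes the Box, and strips camera and light from Movable objects.
; Highlighting toggles an overlay material along with Nanite disallowance.
; Inspecting Static objects animates camera FOV via timeline, then flickers the RectLight on; stopping turns it off.
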(event `self.ReceiveBeginPlay`
  (`self.UpdateOnStart`
    (:`then`
      (`self.Update`)
      (set `StaticMeshComponent.bDisallowNanite` false (`self.StaticMesh`)))
    (:`else`)))

(event `Update`
  (bind (_objectdata_name _objectdata_type) (break `/Game/Systeme/Clue/Struct/F_InteractObject` (`self.ObjectData`)))
  (bind (_objectdata_name_2 _objectdata_type_2 _objectdata_mesh _objectdata_hasclue _objectdata_clue) (break `/Game/Systeme/Clue/Struct/F_InteractObject` (`self.ObjectData`)))
  (if (`|EnumInequality` (`self.ObjectName`) "NewEnumerator5")
    (bind (_objectdata _sucses) (`/Game/BP/BPL_General.getObjectDataByName` (`self.ObjectName`)))
    (set `self.ObjectData` _objectdata)
    (if _sucses
      (bind (_name _type _mesh _hasclue) (break `/Game/Systeme/Clue/Struct/F_InteractObject` _objectdata))
      (`StaticMeshComponent.SetStaticMesh` (`self.StaticMesh`) _mesh)
      (`BoxComponent.SetBoxExtent` (`self.Box`) (`KismetMathLibrary.ClampVectorSize` (`.BoxExtent` (`KismetSystemLibrary.GetComponentBounds` (`self.StaticMesh`))) 5.0 1000.0) true)
      (`|ExecutionSequence`
        (:`then_0`
          (bind _output_get (set `self.HasClue` _hasclue))
          (if _output_get
            (set `self.ObjectDataClue` _objectdata_clue)))
        (:`then_1`
          (`SceneComponent.K2_SetWorldRotation` :`self` (`self.Box`))
          (`PrimitiveComponent.AddImpulse` (`self.Box`) (`self.Force`) "None" false))
        (:`then_2`
          (switch `/Game/Systeme/Clue/Enum/E_ObjectInteractableType` _objectdata_type
            (:`NewEnumerator0`
              (bind _rectlight (`self.RectLight`)
                (:`then`
                  (bind _camera (`self.Camera`)
                    (:`then`
                      (`ActorComponent.K2_DestroyComponent` _camera)
                      (`ActorComponent.K2_DestroyComponent` _rectlight))
                    (:`else`)))
                (:`else`)))))))
    (else
      (`self.K2_DestroyActor`))))

(event `/Game/BP/BPI_Interactable.StartOverlay`
  (set `StaticMeshComponent.bDisallowNanite` true (`self.StaticMesh`))
  (`MeshComponent.SetOverlayMaterial` (`self.StaticMesh`) "/Game/Mat/MI_Overlay_Inst.MI_Overlay_Inst"))

(event `OnBeginCursorOver_Event` :!signature `self.OnBeginCursorOver`
  (params (TouchedActor :type "Actor Object Reference")))

(event `/Game/BP/BPI_Interactable.StopOverlay`
  (set `StaticMeshComponent.bDisallowNanite` false (`self.StaticMesh`))
  (`MeshComponent.SetOverlayMaterial` (`self.StaticMesh`) null))

(event `/Game/BP/BPI_Interactable.StartInspection`
  (bind (_objectdata_name _objectdata_type) (break `/Game/Systeme/Clue/Struct/F_InteractObject` (`self.ObjectData`)))
  (switch `/Game/Systeme/Clue/Enum/E_ObjectInteractableType` _objectdata_type
    (:`NewEnumerator1`
      (set `self.IsInspection` true)
      (set `StaticMeshComponent.bDisallowNanite` false (`self.StaticMesh`))
      (`|ExecutionSequence`
        (:`then_0`
          (bind (_direction _fov) (`Timeline|MOvingCam`)
            (:`Update`
              (`CameraComponent.SetFieldOfView` (`self.Camera`) _fov))))
        (:`then_1`
          (`KismetSystemLibrary.Delay` 1.5)
          (`self.IsInspection`
            (:`then`
              (`LightComponent.SetIntensity` (`self.RectLight`) (`self.LightIntensity`))
              (`KismetSystemLibrary.Delay` 0.2)
              (`LightComponent.SetIntensity` (`self.RectLight`) 25.0)
              (`KismetSystemLibrary.Delay` 0.2)
              (`LightComponent.SetIntensity` (`self.RectLight`) (`self.LightIntensity`))
              (`self.IsInspection`
                (:`then`)
                (:`else`
                  (`LightComponent.SetIntensity` (`self.RectLight`) 0.0))))
            (:`else`)))))))

(event `/Game/BP/BPI_Interactable.StopInspection`
  (bind (_objectdata_name _objectdata_type) (break `/Game/Systeme/Clue/Struct/F_InteractObject` (`self.ObjectData`)))
  (set `self.IsInspection` false)
  (set `StaticMeshComponent.bDisallowNanite` true (`self.StaticMesh`))
  (switch `/Game/Systeme/Clue/Enum/E_ObjectInteractableType` _objectdata_type
    (:`NewEnumerator1`
      (`LightComponent.SetIntensity` (`self.RectLight`) 0.0))))

(fn `GetData`
  (returns (ObjectData :type "/Game/Systeme/Clue/Struct/F_InteractObject Structure"))
  (return (`self.ObjectData`)))

(fn `UserConstructionScript`)