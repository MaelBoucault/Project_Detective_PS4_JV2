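; Light actor Blueprint that fades its RectLight in at start and makes it glitch periodically.
; A looping timer steps intensity up in fixed increments until it reaches MaxIntensity.
; A second looping timer, its period randomized once at BeginPlay from IntervalBugLitgh, runs BugLight.
; BugLight flickers the light twice between BugIntensity and MaxIntensity using random delays, independently of the fade-in value.
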(event `self.ReceiveBeginPlay`
  (bind (_intervalbuglitgh_x _intervalbuglitgh_y) (`KismetMathLibrary.BreakVector2D` (`self.IntervalBugLitgh`)))
  (`KismetSystemLibrary.K2_SetTimerDelegate` (delegate `SetIntensity`) 0.2 true)
  (`KismetSystemLibrary.K2_SetTimerDelegate` (delegate `BugLight`) (`KismetMathLibrary.RandomFloatInRange` _intervalbuglitgh_x _intervalbuglitgh_y) true))

(event `BugLight`
  (`LightComponent.SetIntensity` (`self.RectLight`) (`self.BugIntensity`))
  (`KismetSystemLibrary.Delay` (`KismetMathLibrary.RandomFloatInRange` 0.1 1.0))
  (`LightComponent.SetIntensity` (`self.RectLight`) (`self.MaxIntensity`))
  (`LightComponent.SetIntensity` (`self.RectLight`) (`self.BugIntensity`))
  (`KismetSystemLibrary.Delay` (`KismetMathLibrary.RandomFloatInRange` 0.3 1.0))
  (`LightComponent.SetIntensity` (`self.RectLight`) (`self.MaxIntensity`)))

(event `SetIntensity`
  (bind _rectlight (`self.RectLight`))
  (bind _returnvalue (+ (`self.CurrentIntensity`) 0.5))
  (if (< (`self.CurrentIntensity`) (`self.MaxIntensity`))
    (if (< _returnvalue (`self.MaxIntensity`))
      (bind _output_get (set `self.CurrentIntensity` _returnvalue))
      (`LightComponent.SetIntensity` _rectlight _output_get)
      (else
        (`LightComponent.SetIntensity` _rectlight (`self.MaxIntensity`))))))

(fn `UserConstructionScript`)