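; Static interactable object for a detective game that can be highlighted and inspected.
; On BeginPlay it loads its data by ObjectName, or destroys itself if that name is the excluded enum value.
; Overlay events swap the highlight material and toggle the mesh's DisallowNanite flag.
; With UseCam, inspection flags the DetectiveController, zooms camera FOV through a timeline and flickers on a delayed RectLight; stopping clears the light and restores movement and aim.
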(event `self.ReceiveBeginPlay`
  (if (`|EnumInequality` (`self.ObjectName`) "NewEnumerator5")
    (bind _objectdata (`/Game/BP/BPL_General.getObjectDataByName` (`self.ObjectName`)))
    (set `self.ObjectData` _objectdata)
    (else
      (`self.K2_DestroyActor`))))

(event `/Game/BP/BPI_Interactable.StartOverlay`
  (bind _staticmesh (`self.StaticMesh`))
  (set `StaticMeshComponent.bDisallowNanite` false _staticmesh)
  (`MeshComponent.SetOverlayMaterial` _staticmesh "/Game/Mat/M_Overlay_Inst.M_Overlay_Inst"))

(event `/Game/BP/BPI_Interactable.StopOverlay`
  (bind _staticmesh (`self.StaticMesh`))
  (set `StaticMeshComponent.bDisallowNanite` true _staticmesh)
  (`MeshComponent.SetOverlayMaterial` _staticmesh null))

(event `self.StartInspection`
  (`self.UseCam`
    (:`then`
      (set `/Game/Player/BP/BP_PlayerController.OnStaticObject` true (`/Game/BP/BPL_General.GetDetectiveController`))
      (set `self.IsInspection` true)
      (`|ExecutionSequence`
        (:`then_0`
          (bind (_direction _fov) (`Timeline|Timeline`)
            (:`Update`
              (`CameraComponent.SetFieldOfView` (`self.Camera`) (* _fov (`self.IntensityZoom`))))))
        (:`then_1`
          (`KismetSystemLibrary.Delay` 1.5)
          (`self.IsInspection`
            (:`then`
              (`LightComponent.SetIntensity` (`self.RectLight`) (`self.LightIntensity`))
              (`KismetSystemLibrary.Delay` 0.2)
              (`LightComponent.SetIntensity` (`self.RectLight`) 25.0)
              (`KismetSystemLibrary.Delay` 0.2)
              (`LightComponent.SetIntensity` (`self.RectLight`) (`self.LightIntensity`))
              (`self.IsInspection`
                (:`then`)
                (:`else`
                  (`LightComponent.SetIntensity` (`self.RectLight`) 0.0))))
            (:`else`)))
        (:`then_2`
          (`self.UseCam`
            (:`then`)
            (:`else`
              (set `/Game/Player/BP/BP_PlayerController.Interact` false (`/Game/BP/BPL_General.GetDetectiveController`)))))))
    (:`else`
      (`/Game/BP/BPL_General.SetCanMoveAndAim` true true))))

(event `self.StopInspection`
  (set `self.IsInspection` false)
  (`LightComponent.SetIntensity` (`self.RectLight`) 0.0)
  (`/Game/BP/BPL_General.SetCanMoveAndAim` true true))

(fn `GetData`
  (returns (ObjectData :type "/Game/Systeme/Clue/Struct/F_InteractObject Structure"))
  (return (`self.ObjectData`)))

(fn `UserConstructionScript`)