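; BP_ArmoirKeys is an inspectable key pickup, apparently for an armoire, that joins the detective's items when inspected.
; StartInspection runs the parent logic, starts the pickup animation and adds the item through the detective controller.
; The TakeAnim timeline pulls the half-scaled actor from its current location toward a point above the player.
; Input is disabled and the HUD interact prompt hidden during the flight, then input returns and the actor is destroyed.
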(event `self.StartInspection`
  (`parent.StartInspection`)
  (`self.Anim`)
  (`/Game/Player/BP/BP_PlayerController.AddItem` (`/Game/BP/BPL_General.GetDetectiveController`) "NewEnumerator2"))

(event `Anim`
  (bind (_returnvalue_x _returnvalue_y _returnvalue_z) (`KismetMathLibrary.BreakVector` (`self.K2_GetActorLocation` (`GameplayStatics.GetPlayerPawn` 0))))
  (`self.DisableInput` (`GameplayStatics.GetPlayerController` 0))
  (bind (_direction _alpha) (`Timeline|TakeAnim` :!via `PlayFromStart`)
    (:`Update`
      (`/Game/UI/WBP_BaseHUD.StopShowInteract` (`/Game/BP/BPL_General.GetDetectiveHUD`))
      (`self.K2_SetActorTransform` (`KismetMathLibrary.MakeTransform` (`KismetMathLibrary.VLerp` (`self.K2_GetActorLocation`) (`KismetMathLibrary.MakeVector` _returnvalue_x _returnvalue_y (+ _returnvalue_z 100.0)) _alpha) (struct) (0.5 0.5 0.5)))
      (`/Game/UI/WBP_BaseHUD.StopShowInteract` (`/Game/BP/BPL_General.GetDetectiveHUD`)))
    (:`Finished`
      (`/Game/UI/WBP_BaseHUD.StopShowInteract` (`/Game/BP/BPL_General.GetDetectiveHUD`))
      (`self.EnableInput` (`GameplayStatics.GetPlayerController` 0))
      (`self.K2_DestroyActor`))))

(fn `UserConstructionScript`
  (`parent.UserConstructionScript`))