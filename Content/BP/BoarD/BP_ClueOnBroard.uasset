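; Clue actor pinned on a board, showing the icon from its clue data on a plane.
; On BeginPlay it creates a dynamic material for that icon and slightly randomizes the plane's position.
; Overlay events toggle a hover material, and Anim adds a small random roll and pitch to the plane.
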(event `self.ReceiveBeginPlay`
  (bind _plane (`self.Plane`))
  (bind (_data_name _data_desctiption _data_category _data_forwhom_ _data_icon) (break `/Game/Systeme/Clue/Struct/F_Clue` (`/Game/BP/Data/BP_DA_Clue.Data` (`self.Clue`))))
  (bind _returnvalue (`PrimitiveComponent.CreateDynamicMaterialInstance` (`self.Plane`) 0 "/Game/Mat/MM_ClueOnBoard.MM_ClueOnBoard" "None"))
  (`MaterialInstanceDynamic.SetTextureParameterValue` _returnvalue "Icon" _data_icon)
  (`SceneComponent.K2_SetWorldLocation` _plane (+ (`SceneComponent.K2_GetComponentLocation` _plane) (`KismetMathLibrary.MakeVector` (`KismetMathLibrary.RandomFloatInRange` 0.0 0.05) (`KismetMathLibrary.RandomFloatInRange` 0.0 0.05) (`KismetMathLibrary.RandomFloatInRange` 0.0 0.05))) false false))

(event `/Game/BP/BPI_Interactable.StartOverlay`
  (`MeshComponent.SetOverlayMaterial` (`self.Plane`) "/Engine/VREditor/LaserPointer/HoverMaterial.HoverMaterial"))

(event `/Game/BP/BPI_Interactable.StopOverlay`
  (`MeshComponent.SetOverlayMaterial` (`self.Plane`) null))

(event `Anim`
  (bind _plane (`self.Plane`))
  (`SceneComponent.K2_SetRelativeRotation` _plane (`KismetMathLibrary.ComposeRotators` (`SceneComponent.RelativeRotation` _plane) (`KismetMathLibrary.MakeRotator` (`KismetMathLibrary.RandomFloatInRange` -1.0 1.0) (`KismetMathLibrary.RandomFloatInRange` -0.2 0.2))) false false))

(fn `GetData`
  (returns (ObjectData :type "/Game/Systeme/Clue/Struct/F_InteractObject Structure"))
  (return))

(fn `UserConstructionScript`)