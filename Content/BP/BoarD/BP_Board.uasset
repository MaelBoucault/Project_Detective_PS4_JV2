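; BP_Board is a detective clue board that starts with six character description clues pinned to it.
; AddClue spawns a BP_ClueOnBroard actor per clue data asset, attaches it to the root, scatters it randomly in Y/Z around SpawnClue within set ranges, then calls its Anim.
; A box trigger shows the detective HUD's interact prompt and sets InFrontOfBoard on the controller while the detective pawn overlaps it.
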(event `self.ReceiveBeginPlay`
  (`self.Init`))

(event `Init`
  (`self.AddClue` "/Game/Data/SuspectDescription/DA_Camille_Description.DA_Camille_Description")
  (`self.AddClue` "/Game/Data/SuspectDescription/DA_Gregorette_Description.DA_Gregorette_Description")
  (`self.AddClue` "/Game/Data/SuspectDescription/DA_Jerome_Description.DA_Jerome_Description")
  (`self.AddClue` "/Game/Data/SuspectDescription/DA_Milo_Description.DA_Milo_Description")
  (`self.AddClue` "/Game/Data/SuspectDescription/DA_Timeo_Description.DA_Timeo_Description")
  (`self.AddClue` "/Game/Data/SuspectDescription/DA_Tom_Description.DA_Tom_Description"))

(event `self.Box.OnComponentBeginOverlap`
  (params (OverlappedComponent :type "PrimitiveComponent Object Reference") (OtherActor :type "Actor Object Reference") (OtherComp :type "PrimitiveComponent Object Reference") (OtherBodyIndex :type Integer) (bFromSweep :type Boolean) (SweepResult :type "HitResult Structure (by ref)"))
  (if (== OtherActor (`/Game/BP/BPL_General.GetDetectivePawn`))
    (`/Game/UI/WBP_BaseHUD.StartShowInteract` (`/Game/BP/BPL_General.GetDetectiveHUD`) (make `/Game/UI/Struct/F_InputInteraction` "E"))
    (set `/Game/Player/BP/BP_PlayerController.InFrontOfBoard` true (`/Game/BP/BPL_General.GetDetectiveController`))))

(event `self.Box.OnComponentEndOverlap`
  (params (OverlappedComponent :type "PrimitiveComponent Object Reference") (OtherActor :type "Actor Object Reference") (OtherComp :type "PrimitiveComponent Object Reference") (OtherBodyIndex :type Integer))
  (if (== (`/Game/BP/BPL_General.GetDetectivePawn`) OtherActor)
    (`/Game/UI/WBP_BaseHUD.StopShowInteract` (`/Game/BP/BPL_General.GetDetectiveHUD`))
    (set `/Game/Player/BP/BP_PlayerController.InFrontOfBoard` false (`/Game/BP/BPL_General.GetDetectiveController`))))

(event `AddClue`
  (params (Clue :type "/Game/BP/Data/BP_DA_Clue Object Reference"))
  (bind (_rangespawncluey_x _rangespawncluey_y) (`KismetMathLibrary.BreakVector2D` (`self.RangeSpawnClueY`)))
  (bind (_rangespawncluez_x _rangespawncluez_y) (`KismetMathLibrary.BreakVector2D` (`self.RangeSpawnClueZ`)))
  (bind _returnvalue (`SceneComponent.GetRelativeTransform` (`self.SpawnClue`)))
  (bind _returnvalue_2 (`|SpawnActorFromClass` "/Game/BP/BoarD/BP_ClueOnBroard.BP_ClueOnBroard_C" (`KismetMathLibrary.MakeTransform` (0.0 0.0 0.0)) "Undefined" "MultiplyWithRoot" null "/Game/Mat/MM_ClueOnBoard.MM_ClueOnBoard" Clue null))
  (`self.K2_AttachToComponent` _returnvalue_2 (`self.DefaultSceneRoot`) "None" "SnapToTarget" "SnapToTarget" "SnapToTarget" true)
  (`self.K2_SetActorRelativeTransform` _returnvalue_2 (`KismetMathLibrary.MakeTransform` (`KismetMathLibrary.MakeVector` (.x (.location _returnvalue)) (+ (`KismetMathLibrary.RandomFloatInRange` _rangespawncluey_x _rangespawncluey_y) (.y (.location _returnvalue))) (+ (`KismetMathLibrary.RandomFloatInRange` _rangespawncluez_x _rangespawncluez_y) (.z (.location _returnvalue)))) (.rotation _returnvalue) (.scale _returnvalue)) false true)
  (`/Game/BP/BoarD/BP_ClueOnBroard.Anim` _returnvalue_2))

(fn `UserConstructionScript`)