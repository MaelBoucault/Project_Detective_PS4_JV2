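; BP_BoardMenu is a 3D board menu actor with post-its, an audio mute icon, an inputs panel and a solution notebook.
; Custom events toggle component visibility to show inputs, the brush panel, the solution alert and mute state.
; The notebook animates open and closed, with delays timing its pages, which flip between two spreads.
; BeginPlay hides panels, applies the mute setting and collects eight post-its, whose world locations GetLocPostiit returns by index.
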(event `Mute`
  (`SceneComponent.SetVisibility` (`self.AudioLogoMute`) true false)
  (`SceneComponent.SetVisibility` (`self.AudioLogo`) false false))

(event `Unmute`
  (`SceneComponent.SetVisibility` (`self.AudioLogoMute`) false false)
  (`SceneComponent.SetVisibility` (`self.AudioLogo`) true false))

(event `CloseSolution`
  (`SceneComponent.SetVisibility` (`self.page1`) false false)
  (`SceneComponent.SetVisibility` (`self.page2`) false false)
  (`SceneComponent.SetVisibility` (`self.page3`) false false)
  (`SceneComponent.SetVisibility` (`self.page4`) false false)
  (`GeometryCacheComponent.PlayReversedFromEnd` (`self.GC_MenuNotebook1`))
  (`KismetSystemLibrary.Delay` 0.7)
  (`SceneComponent.SetVisibility` (`self.GC_MenuNotebook1`) false false))

(event `AlertSolu`
  (bind _back (`self.Back`))
  (bind (_relativescale3d_x _relativescale3d_y _relativescale3d_z) (`KismetMathLibrary.BreakVector` (`SceneComponent.RelativeScale3D` _back)))
  (`SceneComponent.SetVisibility` (`self.AlertSolution`) true false)
  (`SceneComponent.SetVisibility` (`self.ToMenu`) true false)
  (`SceneComponent.SetVisibility` (`self.SM_Postit_Touches`) true false)
  (`SceneComponent.SetVisibility` _back true false)
  (`SceneComponent.SetRelativeScale3D` _back (`KismetMathLibrary.MakeVector` 0.01 _relativescale3d_y _relativescale3d_z)))

(event `CloseAlert`
  (`SceneComponent.SetVisibility` (`self.AlertSolution`) false false)
  (`SceneComponent.SetVisibility` (`self.ToMenu`) false false)
  (`SceneComponent.SetVisibility` (`self.SM_Postit_Touches`) false false)
  (`SceneComponent.SetVisibility` (`self.Back`) false false))

(event `BackPage`
  (`SceneComponent.SetVisibility` (`self.page4`) false false)
  (`SceneComponent.SetVisibility` (`self.page3`) false false)
  (`SceneComponent.SetVisibility` (`self.page2`) true false)
  (`SceneComponent.SetVisibility` (`self.GC_MenuNotebook1`) true false)
  (`SceneComponent.SetVisibility` (`self.page1`) true false))

(event `ForwardPage`
  (`SceneComponent.SetVisibility` (`self.GC_MenuNotebook1`) true false)
  (`SceneComponent.SetVisibility` (`self.page4`) true false)
  (`SceneComponent.SetVisibility` (`self.page3`) true false)
  (`SceneComponent.SetVisibility` (`self.page2`) false false)
  (`SceneComponent.SetVisibility` (`self.page1`) false false))

(event `OpenSolution`
  (`SceneComponent.SetVisibility` (`self.AlertSolution`) false false)
  (`SceneComponent.SetVisibility` (`self.ToMenu`) false false)
  (`SceneComponent.SetVisibility` (`self.SM_Postit_Touches`) false false)
  (`SceneComponent.SetVisibility` (`self.Back`) false false)
  (`SceneComponent.SetVisibility` (`self.GC_MenuNotebook1`) true false)
  (`GeometryCacheComponent.PlayFromStart` (`self.GC_MenuNotebook1`))
  (`KismetSystemLibrary.Delay` 0.6)
  (`SceneComponent.SetVisibility` (`self.page1`) true false)
  (`SceneComponent.SetVisibility` (`self.page2`) true false))

(event `UnshowPinceau`
  (`SceneComponent.SetVisibility` (`self.Back`) false false)
  (`SceneComponent.SetVisibility` (`self.SM_Postit_Touches`) false false))

(event `ShowPinceau`
  (`SceneComponent.SetVisibility` (`self.Back`) true false)
  (`SceneComponent.SetVisibility` (`self.SM_Postit_Touches`) true false))

(event `UnshowInputs`
  (`SceneComponent.SetVisibility` (`self.SM_Postit_Touches`) false false)
  (`SceneComponent.SetVisibility` (`self.Touches`) false false)
  (`SceneComponent.SetVisibility` (`self.Back`) false false))

(event `ShowInputs`
  (bind _back (`self.Back`))
  (bind (_relativescale3d_x _relativescale3d_y _relativescale3d_z) (`KismetMathLibrary.BreakVector` (`SceneComponent.RelativeScale3D` _back)))
  (`SceneComponent.SetVisibility` (`self.SM_Postit_Touches`) true false)
  (`SceneComponent.SetVisibility` (`self.Touches`) true false)
  (`SceneComponent.SetVisibility` _back true false)
  (`SceneComponent.SetRelativeScale3D` _back (`KismetMathLibrary.MakeVector` 0.01 _relativescale3d_y _relativescale3d_z)))

(event `self.ReceiveBeginPlay`
  (bind _bp_postit_child_2 (`self.BP Postit Child 2`))
  (bind _back (`self.Back`))
  (bind _audiologomute (`self.AudioLogoMute`))
  (bind _audiologo (`self.AudioLogo`))
  (bind (_relativescale3d_x _relativescale3d_y _relativescale3d_z) (`KismetMathLibrary.BreakVector` (`SceneComponent.RelativeScale3D` _back)))
  (`KismetArrayLibrary.Array_Add` _bp_postit_child_2 (`self.BP_Postit`))
  (`KismetArrayLibrary.Array_Add` _bp_postit_child_2 (`self.BP_Postit1`))
  (`KismetArrayLibrary.Array_Add` _bp_postit_child_2 (`self.BP_Postit2`))
  (`KismetArrayLibrary.Array_Add` _bp_postit_child_2 (`self.BP_Postit3`))
  (`KismetArrayLibrary.Array_Add` _bp_postit_child_2 (`self.BP_Postit4`))
  (`KismetArrayLibrary.Array_Add` _bp_postit_child_2 (`self.BP_Postit5`))
  (`KismetArrayLibrary.Array_Add` _bp_postit_child_2 (`self.BP_Postit6`))
  (`KismetArrayLibrary.Array_Add` _bp_postit_child_2 (`self.BP_Postit7`))
  (`SceneComponent.SetVisibility` (`self.SM_Postit_Touches`) false false)
  (`SceneComponent.SetVisibility` (`self.Touches`) false false)
  (`SceneComponent.SetVisibility` (`self.Back`) false false)
  (`SceneComponent.SetVisibility` (`self.GC_MenuNotebook1`) false false)
  (`SceneComponent.SetVisibility` (`self.page2`) false false)
  (`SceneComponent.SetVisibility` (`self.page3`) false false)
  (`SceneComponent.SetVisibility` (`self.page4`) false false)
  (`SceneComponent.SetVisibility` (`self.page1`) false false)
  (`SceneComponent.SetVisibility` (`self.ToMenu`) false false)
  (`SceneComponent.SetVisibility` (`self.AlertSolution`) false false)
  (`SceneComponent.SetVisibility` (`self.AudioLogoMute`) false false)
  (`SceneComponent.SetRelativeScale3D` _back (`KismetMathLibrary.MakeVector` 0.01 _relativescale3d_y _relativescale3d_z))
  (`SceneComponent.SetRelativeScale3D` (`self.ToMenu`) (`KismetMathLibrary.MakeVector` 0.01 _relativescale3d_y _relativescale3d_z))
  (if (`self.MuteSound`)
    (`SceneComponent.SetVisibility` _audiologo false false)
    (`SceneComponent.SetVisibility` _audiologomute true false)
    (else
      (`SceneComponent.SetVisibility` _audiologo true false)
      (`SceneComponent.SetVisibility` _audiologomute false false))))

(fn `GetLocPostiit`
  (params (index :type Integer))
  (returns (LOc :type "Vector Structure"))
  (return (`SceneComponent.K2_GetComponentLocation` (`|GetArrayItem` (`self.BP Postit Child 2`) index))))

(fn `UserConstructionScript`)