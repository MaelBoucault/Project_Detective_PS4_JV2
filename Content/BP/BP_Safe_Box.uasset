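; Inspectable safe actor that opens when the player enters the correct four-number combination on its dial.
; BeginPlay loads object data by name, or destroys the actor for one enum value, and maps sphere colliders to dial numbers.
; Each press appends a number and requests dial rotation; the fourth triggers a code check that swings the door open or clears the entry.
; Inspection animates camera FOV and flickers a light; an overlay material provides highlighting.
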(event `Open`
  (`self.IsOpen`
    (:`then`)
    (:`else`
      (set `self.IsOpen` true)
      (bind (_direction _axe) (`Timeline|Opendoor` :!via `PlayFromStart`)
        (:`Update`
          (`SceneComponent.K2_SetRelativeRotation` (`self.SM_Safe_Door`) (`KismetMathLibrary.MakeRotator` 0.0 0.0 _axe) false false))))))

(event `self.ReceiveBeginPlay`
  (if (`|EnumInequality` (`self.ObjectName`) "NewEnumerator5")
    (`|ExecutionSequence`
      (:`then_0`
        (bind _objectdata (`/Game/BP/BPL_General.getObjectDataByName` (`self.ObjectName`)))
        (set `self.Object Data` _objectdata))
      (:`then_1`
        (`self.Init`)))
    (else
      (`self.K2_DestroyActor`))))

(event `/Game/BP/BPI_Interactable.StartInspection`
  (set `self.IsInspection` true)
  (`|ExecutionSequence`
    (:`then_0`
      (bind (_direction _fov) (`Timeline|Timeline`)
        (:`Update`
          (`CameraComponent.SetFieldOfView` (`self.Camera`) _fov))))
    (:`then_1`
      (`KismetSystemLibrary.Delay` 1.5)
      (`self.IsInspection`
        (:`then`
          (`LightComponent.SetIntensity` (`self.RectLight`) (`self.LightIntensity`))
          (`KismetSystemLibrary.Delay` 0.2)
          (`LightComponent.SetIntensity` (`self.RectLight`) 25.0)
          (`KismetSystemLibrary.Delay` 0.2)
          (`LightComponent.SetIntensity` (`self.RectLight`) (`self.LightIntensity`))
          (`self.IsInspection`
            (:`then`)
            (:`else`
              (`LightComponent.SetIntensity` (`self.RectLight`) 0.0))))
        (:`else`)))))

(event `/Game/BP/BPI_Interactable.StartOverlay`
  (`MeshComponent.SetOverlayMaterial` (`self.SM_Safe_Door`) "/Game/Mat/M_Overlay_Inst.M_Overlay_Inst")
  (`MeshComponent.SetOverlayMaterial` (`self.SM_Safe_Box`) "/Game/Mat/M_Overlay_Inst.M_Overlay_Inst"))

(event `/Game/BP/BPI_Interactable.StopOverlay`
  (`MeshComponent.SetOverlayMaterial` (`self.SM_Safe_Door`) null)
  (`MeshComponent.SetOverlayMaterial` (`self.SM_Safe_Box`) null))

(event `RotateLockByAngle`
  (params (Angle :type Integer))
  (bind _returnvalue (`KismetMathLibrary.Conv_IntToDouble` Angle))
  (set `self.RotationAngle` (`KismetMathLibrary.RandomFloatInRange` (+ _returnvalue 0.05) (- _returnvalue 0.05)))
  (`TimelineComponent.PlayFromStart` (`self.Rotate`)))

(event `/Game/BP/BPI_Interactable.StopInspection`
  (set `self.IsInspection` false)
  (`LightComponent.SetIntensity` (`self.RectLight`) 0.0)
  (`/Game/BP/BPL_General.SetCanMoveAndAim` true true))

(fn `AddNumberToCurrentCode`
  (params (Number :type "Integer (by ref)"))
  (returns (CodeLength :type Integer))
  (bind _currentcode (`self.CurrentCode`))
  (if (<= (`KismetArrayLibrary.Array_Length` (`self.CurrentCode`)) 4)
    (`self.RestCurrentCode`))
  (`KismetArrayLibrary.Array_Add` _currentcode (`local.Number`))
  (return (`KismetArrayLibrary.Array_Length` _currentcode)))

(fn `GetAngleRotation`
  (params (Number :type Integer))
  (returns (Angle :type Integer))
  (return (/ (* Number 360) 40)))

(fn `GetData`
  (returns (ObjectData :type "/Game/Systeme/Clue/Struct/F_InteractableObject Structure"))
  (return (`self.Object Data`)))

(fn `GetNumberByCollision`
  (params (Collision :type "PrimitiveComponent Object Reference"))
  (returns (Number :type Integer))
  (bind (_keypin _valuepin) (`|MapForEach` (`self.CollisionToNumber`))
    (:`then`
      (if (`KismetStringLibrary.EqualEqual_StrStr` (`KismetSystemLibrary.GetObjectName` _keypin) (`KismetSystemLibrary.GetObjectName` Collision))
        (return _valuepin)))
    (:`CompletedPin`
      (`KismetSystemLibrary.PrintString` "Collision_Don't_Have_Number"))))

(fn `Init`
  (`BlueprintMapLibrary.Map_Add` (`self.CollisionToNumber`) (`self.00_Sphere`))
  (`BlueprintMapLibrary.Map_Add` (`self.CollisionToNumber`) (`self.05_Sphere`) 5)
  (`BlueprintMapLibrary.Map_Add` (`self.CollisionToNumber`) (`self.10_Sphere`) 10)
  (`BlueprintMapLibrary.Map_Add` (`self.CollisionToNumber`) (`self.15_Sphere`) 15)
  (`BlueprintMapLibrary.Map_Add` (`self.CollisionToNumber`) (`self.20_Sphere`) 20)
  (`BlueprintMapLibrary.Map_Add` (`self.CollisionToNumber`) (`self.25_Sphere`) 25)
  (`BlueprintMapLibrary.Map_Add` (`self.CollisionToNumber`) (`self.30_Sphere`) 30)
  (`BlueprintMapLibrary.Map_Add` (`self.CollisionToNumber`) (`self.35_Sphere`) 35))

(fn `PlayerPressButtun`
  (params (Sphere_Collision :type "PrimitiveComponent Object Reference"))
  (bind _currentcode (`self.CurrentCode`))
  (`self.IsOpen`
    (:`then`)
    (:`else`
      (bind _number (`self.GetNumberByCollision` Sphere_Collision))
      (`KismetArrayLibrary.Array_Add` _currentcode _number)
      (`|ExecutionSequence`
        (:`then_0`
          (bind _angle (`self.GetAngleRotation` _number))
          (`self.RotateLockByAngle` _angle))
        (:`then_1`
          (if (>= (`KismetArrayLibrary.Array_Length` _currentcode) 4)
            (bind _goodcode (`self.VerifCode`))
            (if _goodcode
              (`self.Open`)
              (else
                (`self.RestCurrentCode`)))))))))

(fn `RestCurrentCode`
  (`KismetArrayLibrary.Array_Clear` (`self.CurrentCode`)))

(fn `UserConstructionScript`)

(fn `VerifCode`
  (returns (goodCode :type Boolean))
  (return (`KismetArrayLibrary.Array_Identical` (`self.RealCode`) (`self.CurrentCode`))))