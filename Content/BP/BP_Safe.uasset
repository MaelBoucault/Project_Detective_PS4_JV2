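; BP_Safe is an inspectable safe actor that loads its object data by name on BeginPlay, or destroys itself for one specific name value.
; StartInspection animates camera FOV, flickers a rect light after a delay and swings the door open, using timelines for FOV and door yaw.
; Overlay events toggle a highlight material on door and box, and GetData exposes the loaded data.
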(event `self.ReceiveBeginPlay`
  (if (`|EnumInequality` (`self.ObjectName`) "NewEnumerator5")
    (bind _objectdata (`/Game/BP/BPL_General.getObjectDataByName` (`self.ObjectName`)))
    (set `self.Object Data` _objectdata)
    (else
      (`self.K2_DestroyActor`))))

(event `/Game/BP/BPI_Interactable.StartInspection`
  (set `self.IsInspection` true)
  (`|ExecutionSequence`
    (:`then_0`
      (bind (_direction _fov) (`Timeline|Timeline`)
        (:`Update`
          (`CameraComponent.SetFieldOfView` (`self.Camera`) _fov))))
    (:`then_1`
      (`KismetSystemLibrary.Delay` 1.5)
      (`self.IsInspection`
        (:`then`
          (`LightComponent.SetIntensity` (`self.RectLight`) (`self.LightIntensity`))
          (`KismetSystemLibrary.Delay` 0.2)
          (`LightComponent.SetIntensity` (`self.RectLight`) 25.0)
          (`KismetSystemLibrary.Delay` 0.2)
          (`LightComponent.SetIntensity` (`self.RectLight`) (`self.LightIntensity`))
          (`self.IsInspection`
            (:`then`)
            (:`else`
              (`LightComponent.SetIntensity` (`self.RectLight`) 0.0))))
        (:`else`)))
    (:`then_2`
      (`self.Open`))))

(event `/Game/BP/BPI_Interactable.StartOverlay`
  (`MeshComponent.SetOverlayMaterial` (`self.SM_Safe_Door`) "/Game/Mat/M_Overlay_Inst.M_Overlay_Inst")
  (`MeshComponent.SetOverlayMaterial` (`self.SM_Safe_Box`) "/Game/Mat/M_Overlay_Inst.M_Overlay_Inst"))

(event `/Game/BP/BPI_Interactable.StopOverlay`
  (`MeshComponent.SetOverlayMaterial` (`self.SM_Safe_Door`) null)
  (`MeshComponent.SetOverlayMaterial` (`self.SM_Safe_Box`) null))

(event `Open`
  (bind (_direction _axe) (`Timeline|Opendoor` :!via `PlayFromStart`)
    (:`Update`
      (`SceneComponent.K2_SetRelativeRotation` (`self.SM_Safe_Door`) (`KismetMathLibrary.MakeRotator` 0.0 0.0 _axe) false false))))

(fn `GetData`
  (returns (ObjectData :type "/Game/Systeme/Clue/Struct/F_InteractableObject Structure"))
  (return (`self.Object Data`)))

(fn `UserConstructionScript`)