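; Interactable drawer for a detective game that slides open and closed, with an overlay material highlight.
; On BeginPlay it picks one of three mesh variants, optionally spawns an interactable object inside and can start open.
; Anim toggles a timeline slide; when a key is needed, the great and coffee-table variants check the detective controller's items.
; A missing key plays a buzz and a pitch animation instead.
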(event `/Game/BP/BPI_Interactable.StartOverlay`
  ;[0.15 0.15 0.15 0.5 106] Overlay
  (`MeshComponent.SetOverlayMaterial` (`self.SM_Drawer`) "/Game/Mat/MI_Overlay_Inst.MI_Overlay_Inst"))

(event `/Game/BP/BPI_Interactable.StopOverlay`
  ;[0.15 0.15 0.15 0.5 106] Overlay
  (`MeshComponent.SetOverlayMaterial` (`self.SM_Drawer`) null))

(event `self.ReceiveBeginPlay`
  (bind _sm_drawer (`self.SM_Drawer`))
  (`|ExecutionSequence`
    (:`then_0`
      (`self.GreatDrawer`
        (:`then`
          (`StaticMeshComponent.SetStaticMesh` (`self.SM_Drawer`) "/Game/Meshes/OptimizedDeskMeshes/SM_Drawer_01.SM_Drawer_01")
          (set `self.DrawerHeight` 5.0))
        (:`else`
          (`self.CoffeDrawer`
            (:`then`
              (`StaticMeshComponent.SetStaticMesh` _sm_drawer "/Game/Meshes/SM_Coffee_Table_Bot_Drawer.SM_Coffee_Table_Bot_Drawer")
              (set `self.DrawerHeight` 15.0))
            (:`else`
              (`StaticMeshComponent.SetStaticMesh` _sm_drawer "/Game/Meshes/OptimizedDeskMeshes/SM_Drawer_02.SM_Drawer_02"))))))
    (:`then_1`
      (`self.HasObject`
        (:`then`
          (bind _returnvalue (`|SpawnActorFromClass` "/Game/BP/BP_InteractableObject.BP_InteractableObject_C" (`SceneComponent.K2_GetComponentToWorld` (`self.SpawnObject`)) "Undefined" "MultiplyWithRoot" null (`self.ObjectName`) (0.0 0.0 0.0) null))
          (`/Game/BP/BP_InteractableObject.Update` _returnvalue))
        (:`else`)))
    (:`then_2`
      (`self.OpenOnStart`
        (:`then`
          (`self.Anim`))
        (:`else`)))))

(event `Anim`
  (bind _openanimation (`self.OpenAnimation`))
  (`self.IsAnim`
    (:`then`)
    (:`else`
      (`self.NeedKey`
        (:`then`
          (`self.GreatDrawer`
            (:`then`
              (if (`/Game/Player/BP/BP_PlayerController.HasItem` (`/Game/BP/BPL_General.GetDetectiveController`) "NewEnumerator1")
                (set `self.IsAnim` true :!label _label)
                (`self.Open`
                  (:`then`
                    (`TimelineComponent.Reverse` _openanimation))
                  (:`else`
                    (`TimelineComponent.PlayFromStart` _openanimation)))
                (`GameplayStatics.PlaySound2D` "/Game/Audio/SFX/SC_DrawerOpen_Cue.SC_DrawerOpen_Cue" 1.0 1.0 0.0 null null)
                (else
                  (`self.AnimIsLock` :!label _label_2))))
            (:`else`
              (`self.CoffeDrawer`
                (:`then`
                  (if (`/Game/Player/BP/BP_PlayerController.HasItem` (`/Game/BP/BPL_General.GetDetectiveController`) "NewEnumerator2")
                    (goto _label)
                    (else
                      (goto _label_2))))
                (:`else`
                  (goto _label))))))
        (:`else`
          (goto _label))))))

(event `AnimIsLock`
  (bind _sm_drawer (`self.SM_Drawer`))
  (bind (_relativerotation_roll _relativerotation_pitch _relativerotation_yaw) (`KismetMathLibrary.BreakRotator` (`SceneComponent.RelativeRotation` _sm_drawer)))
  (`GameplayStatics.PlaySound2D` "/Game/Audio/SFX/SC_WrongBuzz_Cue.SC_WrongBuzz_Cue" 0.5 1.0 0.0 null null)
  (bind (_direction _alpha) (`Timeline|Timeline` :!via `PlayFromStart`)
    (:`Update`
      (bind (_returnvalue_roll _returnvalue_pitch) (`KismetMathLibrary.BreakRotator` (`KismetMathLibrary.RLerp` (`self.K2_GetActorRotation`) (`KismetMathLibrary.MakeRotator` 0.0 5.0) _alpha)))
      (`SceneComponent.K2_SetRelativeRotation` _sm_drawer (`KismetMathLibrary.MakeRotator` _relativerotation_roll _returnvalue_pitch _relativerotation_yaw) false false))))

(fn `GetData`
  (returns (ObjectData :type "/Game/Systeme/Clue/Struct/F_InteractableObject Structure"))
  (return (`self.ObjectData`)))

(fn `UserConstructionScript`)