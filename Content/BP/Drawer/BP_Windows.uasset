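; BP_Windows is an interactive window actor that swings open and closed, optionally starting its animation on BeginPlay via OpenOnStart.
; Anim plays or reverses a timeline that yaws Origin between 0 and 90 degrees, with flags blocking retriggers and tracking open state.
; StartOverlay and StopOverlay set and clear an overlay material on the SMDrawer mesh.
; GetData exposes the actor's ObjectData.
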(event `self.ReceiveBeginPlay`
  (`self.OpenOnStart`
    (:`then`
      (`self.Anim`))
    (:`else`)))

(event `Anim`
  (bind _openanimation_0 (`self.OpenAnimation_0`))
  (`self.IsAnim_0`
    (:`then`)
    (:`else`
      (set `self.IsAnim_0` true)
      (`self.Open_0`
        (:`then`
          (`TimelineComponent.Reverse` _openanimation_0))
        (:`else`
          (`TimelineComponent.PlayFromStart` _openanimation_0))))))

(event `self.StartOverlay`
  (`MeshComponent.SetOverlayMaterial` (`self.SM_Drawer`) "/Game/Mat/M_Overlay_Inst.M_Overlay_Inst"))

(event `self.StopOverlay`
  (`MeshComponent.SetOverlayMaterial` (`self.SM_Drawer`) null))

(fn `GetData`
  (returns (ObjectData :type "/Game/Systeme/Clue/Struct/F_InteractObject Structure"))
  (return (`self.ObjectData`)))

(fn `UserConstructionScript`)